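; Gameplay ability that reloads the rifle, allowed only when ammo is below max and reserve remains.
; It plays the reload montage, waits for the reload event, then uses an OnlyServerWait net sync before computing the refill, capped by reserve.
; An effect container deducts reserve through a SetByCaller magnitude, while magazine ammo is set directly on the weapon.
; Montage completion ends the ability after a BothWait sync; interruption cancels it.
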(event `self.K2_ActivateAbility`
  (bind _sourceweapon (`self.SourceWeapon`))
  (bind _sourceweapon_2 (`self.SourceWeapon`))
  (bind _returnvalue (`FCCharacter.GetAmmoReserveAmount` (`self.OwningCharacter`)))
  (`self.InitialCache`)
  (`FCAT_PlayMontageAndWaitForEvent.PlayMontageAndWaitForEvent` "None" "/Game/Animations/StarterPack/MM_Reload_Rifle_Hip_Montage.MM_Reload_Rifle_Hip_Montage" (struct :`GameplayTags` (struct :`(TagName` "Ability.Weapon.Reload")))
    (:`OnCompleted`
      (`AbilityTask_NetworkSyncPoint.WaitNetSync` "BothWait"
        (:`OnSync`
          (`self.K2_EndAbility`))))
    (:`OnInterrupted`
      (`self.K2_CancelAbility` :!label _label))
    (:`OnCancelled`
      (goto _label))
    (:`EventReceived`
      (`AbilityTask_NetworkSyncPoint.WaitNetSync` "OnlyServerWait"
        (:`OnSync`
          (bind _output_get (set `self.ReloadAmount` (- (`FCWeapon.MagazineCapacity` _sourceweapon) (`FCWeapon.GetAmmoAmount` _sourceweapon))))
          (if (<= _output_get _returnvalue)
            (set `self.ActualReloadAmount` _output_get)
            (else
              (set `self.ActualReloadAmount` _returnvalue)))
          (bind _returnvalue_2 (`self.MakeEffectContainerSpec` (struct :`TagName` "Ability") (`self.CurrentEventData`)))
          (`AbilitySystemBlueprintLibrary.AssignTagSetByCallerMagnitude` (`|GetArrayItem` (`.TargetGameplayEffectSpecs` (break `GameplayEffectContainerSpec` _returnvalue_2))) (struct :`TagName` "Data.ReloadAmount.Reserve") (* (`self.ActualReloadAmount`) -1.0))
          (`self.ApplyEffectContainerSpec` _returnvalue_2)
          (`FCWeapon.SetAmmoAmount` _sourceweapon_2 (+ (`FCWeapon.GetAmmoAmount` _sourceweapon_2) (`self.ActualReloadAmount`))))))))

(fn `K2_CanActivateAbility`
  (params (ActorInfo :type "GameplayAbilityActorInfo Structure") (Handle :type "GameplayAbilitySpecHandle Structure"))
  (returns (RelevantTags :type "GameplayTagContainer Structure") (ReturnValue :type Boolean))
  (bind _asfccharacter (cast `FCCharacter` (`.AvatarActor` (break `GameplayAbilityActorInfo` ActorInfo))))
  (return (struct) (and (< (`FCCharacter.GetAmmoAmount` _asfccharacter) (`FCCharacter.GetMaxAmmoAmount` _asfccharacter)) (> (`FCCharacter.GetAmmoReserveAmount` _asfccharacter) 0))))