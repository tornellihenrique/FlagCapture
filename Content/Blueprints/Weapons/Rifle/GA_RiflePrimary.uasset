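; Gameplay ability for the rifle's automatic primary fire, with a short delay when activated while sprinting.
; It activates a cached GA_RiflePrimaryInstant through a batched RPC, then calls its FireBullet on a timed loop for subsequent shots.
; Input release or a failed cost check ends both abilities.
; The cost check requires enough weapon ammo, and on failure triggers the reload ability if this one is inactive.
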(event `self.K2_ActivateAbility`
  (`self.InitialCache`)
  (if (`GameplayTagAssetInterface.HasMatchingGameplayTag` (`self.GetAbilitySystemComponentFromActorInfo`) (struct :`TagName` "State.Sprinting"))
    (`AbilityTask_WaitDelay.WaitDelay` 0.3
      (:`OnFinish`
        _))
    (else
      (`FCAT_WaitDelayOneFrame.WaitDelayOneFrame`
        (:`OnFinish`
          _))))
  (bind _returnvalue (`self.BatchRPCTryActivateAbility` (`self.InstantAbilityHandle`)))
  (if _returnvalue
    ; Tiro Automático
    (`AbilityTask_WaitInputRelease.WaitInputRelease` true
      (:`then`
        (`AbilityTask_WaitDelay.WaitDelay` (`self.TimeBetweenShots`) :!label _label
          (:`OnFinish`
            (bind _returnvalue_2 (`self.K2_CheckAbilityCost`))
            (if _returnvalue_2
              ;; Executa manualmente os tiros após o primeiro
              (`/Game/Blueprints/Weapons/Rifle/GA_RiflePrimaryInstant.FireBullet` (`self.InstantAbility`))
              (goto _label)
              (else
                _)))))
      (:`OnRelease`
        _))
    (`self.K2_EndAbility` (`self.InstantAbility`))
    (`self.K2_EndAbility`)
    (else
      (`self.K2_EndAbility`))))

(fn `MyCheckCost`
  (params (Handle :type "GameplayAbilitySpecHandle Structure") (ActorInfo :type "GameplayAbilityActorInfo Structure (by ref)"))
  (returns (ReturnValue :type Boolean))
  (bind ((`AbilitySystemComponent` _abilitysystemcomponent)) (break `GameplayAbilityActorInfo` (`local.ActorInfo`)))
  (bind _asweapon (cast `FCWeapon` (`self.K2_GetSourceObject` Handle ActorInfo)))
  (if (and (>= (`FCWeapon.GetAmmoAmount` _asweapon) (`self.AmmoCost`)) (`parent.MyCheckCost` Handle ActorInfo))
    (return true)
    (else
      (bind _returnvalue (`FCFunctionLibrary.IsPrimaryAbilityInstanceActive` _abilitysystemcomponent (`local.Handle`)))
      (if (not _returnvalue)
        (`AbilitySystemComponent.TryActivateAbilitiesByTag` _abilitysystemcomponent (`BlueprintGameplayTagLibrary.MakeGameplayTagContainerFromTag` (struct :`TagName` "Ability.Weapon.Reload")) true))
      (return false))))