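; Gameplay ability that switches the owning FCCharacter to its previous weapon.
; It can activate only when the avatar is an FCCharacter carrying more than one weapon.
; On activation it calls PreviousWeapon, applies the GE_WeaponIsChangingDelayReplicationTag effect to the owner, then ends immediately.
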(event `self.K2_ActivateAbility`
  (bind _asfccharacter (cast `FCCharacter` (`self.GetAvatarActorFromActorInfo`)))
  (`FCCharacter.PreviousWeapon` _asfccharacter)
  (`self.BP_ApplyGameplayEffectToOwner` "/Game/Blueprints/Ability/Effects/GE_WeaponIsChangingDelayReplicationTag.GE_WeaponIsChangingDelayReplicationTag_C")
  (`self.K2_EndAbility`))

(fn `K2_CanActivateAbility`
  (params (ActorInfo :type "GameplayAbilityActorInfo Structure") (Handle :type "GameplayAbilitySpecHandle Structure"))
  (returns (RelevantTags :type "GameplayTagContainer Structure") (ReturnValue :type Boolean))
  (bind _asfccharacter (cast `FCCharacter` (`.AvatarActor` (break `GameplayAbilityActorInfo` ActorInfo))))
  (if (> (`FCCharacter.GetNumWeapons` _asfccharacter) 1)
    (return (struct) true)
    (else
      (return (struct) false))))