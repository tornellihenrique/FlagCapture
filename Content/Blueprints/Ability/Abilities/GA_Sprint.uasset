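; Gameplay ability that sprints while input is held, applying a sprint effect, movement-component sprint state and local gameplay cue.
; A short delay loop with server-wait net syncs commits cost only while accelerating and not falling.
; Input release, failed cost or an added Ability.CancelsSprint tag ends the ability.
; Ending briefly applies a removal effect, clears both effects, stops sprinting and removes the cue.
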(event `self.K2_ActivateAbility`
  (bind ((`AbilitySystemComponent` _abilitysystemcomponent) (`MovementComponent` _movementcomponent)) (break `GameplayAbilityActorInfo` (`self.GetActorInfo`)))
  (set `self.EndSprint` false)
  (bind _returnvalue (`self.BP_ApplyGameplayEffectToOwner` "/Game/Blueprints/Ability/Effects/GE_Sprinting.GE_Sprinting_C" (`self.GetAbilityLevel`)))
  (set `self.GE_SprintingHandle` _returnvalue)
  (bind _asfccharacter_movement_component (cast `FCCharacterMovementComponent` _movementcomponent))
  (`FCCharacterMovementComponent.StartSprinting` _asfccharacter_movement_component)
  (bind _asfcability_system_component (cast `FCAbilitySystemComponent` _abilitysystemcomponent))
  (`FCAbilitySystemComponent.AddGameplayCueLocal` :`self` _asfcability_system_component :`GameplayCueTag` (struct :`TagName` "GameplayCue.Ability.Sprinting"))
  (`AbilityTask_WaitInputRelease.WaitInputRelease` true
    (:`then`
      (bind _asynctaskproxy (`AbilityTask_WaitGameplayTagAdded.WaitGameplayTagAdd` (struct :`TagName` "Ability.CancelsSprint") null true)
        (:`then`
          (set `self.WaitCancelsSprintTagAddedTask` _asynctaskproxy)
          (`AbilityTask_WaitDelay.WaitDelay` 0.05 :!label _label
            (:`OnFinish`
              (`AbilityTask_NetworkSyncPoint.WaitNetSync` "OnlyServerWait"
                (:`OnSync`
                  (bind _asfccharacter_movement_component_2 (cast `FCCharacterMovementComponent` (`.MovementComponent` (break `GameplayAbilityActorInfo` (`self.GetActorInfo`)))))
                  (if (and (> (`KismetMathLibrary.VSize` (`CharacterMovementComponent.GetCurrentAcceleration` _asfccharacter_movement_component_2)) 0.0) (not (`NavMovementComponent.IsFalling` _asfccharacter_movement_component_2)))
                    (bind _returnvalue_2 (`self.K2_CommitAbilityCost` false))
                    (if _returnvalue_2
                      (if (not (`self.EndSprint`)) :!label _label_2
                        (goto _label))
                      (else
                        (set `self.EndSprint` true :!label _label_3)
                        (`self.K2_EndAbility`)))
                    (else
                      (goto _label_2))))))))
        (:`Added`
          (`AbilityTask_NetworkSyncPoint.WaitNetSync` "OnlyServerWait"
            (:`OnSync`
              (goto _label_3))))))
    (:`OnRelease`
      (goto _label_3))))

(event `self.K2_OnEndAbility`
  (params (bWasCancelled :type Boolean))
  (bind ((`AbilitySystemComponent` _abilitysystemcomponent) (`MovementComponent` _movementcomponent)) (break `GameplayAbilityActorInfo` (`self.GetActorInfo`)))
  (bind _returnvalue (`self.BP_ApplyGameplayEffectToOwner` "/Game/Blueprints/Ability/Effects/GE_SprintingRemoval.GE_SprintingRemoval_C"))
  (set `self.GE_SprintingRemovalHandle` _returnvalue)
  (`self.BP_RemoveGameplayEffectFromOwnerWithHandle` (`self.GE_SprintingHandle`))
  (`self.BP_RemoveGameplayEffectFromOwnerWithHandle` (`self.GE_SprintingRemovalHandle`))
  (bind _asfccharacter_movement_component (cast `FCCharacterMovementComponent` _movementcomponent))
  (`FCCharacterMovementComponent.StopSprinting` _asfccharacter_movement_component)
  (bind _waitcancelssprinttagaddedtask (`self.WaitCancelsSprintTagAddedTask`)
    (:`then`
      (`GameplayTask.EndTask` _waitcancelssprinttagaddedtask))
    (:`else`
      _))
  (bind _asfcability_system_component (cast `FCAbilitySystemComponent` _abilitysystemcomponent))
  (`FCAbilitySystemComponent.RemoveGameplayCueLocal` :`self` _asfcability_system_component :`GameplayCueTag` (struct :`TagName` "GameplayCue.Ability.Sprinting")))