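; GA_Jump is a gameplay ability that makes the FCCharacterBase avatar jump for as long as input is held.
; On activation it commits the ability, ending it if that fails, then calls Jump on the avatar.
; A WaitInputRelease task ends the ability on release, and OnEndAbility calls StopJumping on the avatar.
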(event `self.K2_ActivateAbility`
  (bind _returnvalue (`self.K2_CommitAbility`))
  (if (not _returnvalue)
    (`self.K2_EndAbility`))
  (bind _asfccharacter_base (cast `FCCharacterBase` (`.AvatarActor` (break `GameplayAbilityActorInfo` (`self.GetActorInfo`)))))
  (`Character.Jump` _asfccharacter_base)
  (`AbilityTask_WaitInputRelease.WaitInputRelease` true
    (:`OnRelease`
      (`self.K2_EndAbility`))))

(event `self.K2_OnEndAbility`
  (params (bWasCancelled :type Boolean))
  (bind _asfccharacter_base (cast `FCCharacterBase` (`.AvatarActor` (break `GameplayAbilityActorInfo` (`self.GetActorInfo`)))))
  (`Character.StopJumping` _asfccharacter_base))