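; BP_CaptureFlag is a capture-the-flag actor that characters carry, with its color showing the holding team.
; The construction script creates a dynamic material in the neutral color, and grabbing snaps the flag to the character's FlagSocket and applies the team color.
; Capture detaches it, restores neutral and returns it to InitialPosition.
; Release does likewise, but moves it to an upward line trace's hit point, resetting only if nothing is hit.
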(event `self.K2_OnGrab`
  (params (Character :type "FCCharacter Object Reference") (Team :type "ETeamSide Enum" :default "None"))
  (`/Engine/EditorBlueprintResources/StandardMacros.IsValid` Character
    (:`Is Valid`
      (`self.K2_AttachToComponent` (`Character.Mesh` Character) "FlagSocket" "SnapToTarget" "SnapToTarget" "KeepRelative")
      (`MaterialInstanceDynamic.SetVectorParameterValue` (`self.Material`) "Color" (`FCFunctionLibrary.GetTeamColor` Team)))))

(event `self.K2_OnCapture`
  (params (Character :type "FCCharacter Object Reference") (Team :type "ETeamSide Enum" :default "None"))
  (`MaterialInstanceDynamic.SetVectorParameterValue` (`self.Material`) "Color" (`self.NeutralColor`))
  (`self.K2_DetachFromActor` "KeepWorld" "KeepWorld" "KeepWorld")
  (`self.K2_SetActorTransform` (`self.InitialPosition`) :!label _label))

(event `self.K2_OnReleased`
  (params (Character :type "FCCharacter Object Reference") (Team :type "ETeamSide Enum" :default "None"))
  (bind _returnvalue (`self.K2_GetActorLocation`))
  (`MaterialInstanceDynamic.SetVectorParameterValue` (`self.Material`) "Color" (`self.NeutralColor`))
  (`self.K2_DetachFromActor` "KeepWorld" "KeepWorld" "KeepWorld")
  (bind (_outhit _returnvalue_2) (`KismetSystemLibrary.LineTraceSingle` _returnvalue (+ _returnvalue (* (0.0 0.0 1.0) 1000.0)) "TraceTypeQuery1"))
  (if _returnvalue_2
    (`self.K2_SetActorLocation` (`.ImpactPoint` (`GameplayStatics.BreakHitResult` _outhit)))
    (else
      (goto _label))))

(fn `UserConstructionScript`
  (bind _returnvalue (`PrimitiveComponent.CreateDynamicMaterialInstance` (`self.StaticMesh`) 0 "/Game/StarterContent/Materials/M_Basic_Wall.M_Basic_Wall" "None"))
  (bind _output_get (set `self.Material` _returnvalue))
  (`MaterialInstanceDynamic.SetVectorParameterValue` _output_get "Color" (`self.NeutralColor`))
  (`PrimitiveComponent.SetMaterial` (`self.StaticMesh`) 0 _output_get))