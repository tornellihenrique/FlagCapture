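; BP_SpawnArea is a team-owned spawn area that serves as an orbiting view target.
; Becoming the view target of a local controller sets Focused, and losing view target clears it.
; While Focused, Tick adds RotationSpeed to TargetYaw without delta-time scaling and applies it as the SpringArm's world yaw.
; The construction script colors and labels the TextRender by owning team, using Portuguese text.
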(event `self.ReceiveTick`
  (params (DeltaSeconds :type "Float (single-precision)"))
  (if (`self.Focused`)
    (bind _output_get (set `self.TargetYaw` (* (+ (`self.TargetYaw`) (`self.RotationSpeed`)) 1.0)))
    (`SceneComponent.K2_SetWorldRotation` (`self.SpringArm`) (`KismetMathLibrary.MakeRotator` (.roll (`SceneComponent.K2_GetComponentRotation` (`self.SpringArm`))) (.pitch (`SceneComponent.K2_GetComponentRotation` (`self.SpringArm`))) _output_get) false false)))

(event `self.K2_OnBecomeViewTarget`
  (params (PC :type "PlayerController Object Reference"))
  (`/Engine/EditorBlueprintResources/StandardMacros.IsValid` PC
    (:`Is Valid`
      (if (`Controller.IsLocalController` PC)
        (set `self.Focused` true)
        (else
          (set `self.Focused` false :!label _label))))
    (:`Is Not Valid`
      (goto _label))))

(event `self.K2_OnEndViewTarget`
  (params (PC :type "PlayerController Object Reference"))
  (set `self.Focused` false))

(fn `UserConstructionScript`
  (`TextRenderComponent.SetTextRenderColor` (`self.TextRender`) (`KismetMathLibrary.Conv_LinearColorToColor` (`FCFunctionLibrary.GetTeamColor` (`self.OwnerTeam`))))
  (`TextRenderComponent.K2_SetText` (`self.TextRender`) (select `ETeamSide` (`self.OwnerTeam`) :`None` "Sem Time" :`Team_A` "Time A" :`Team_B` "Time B")))